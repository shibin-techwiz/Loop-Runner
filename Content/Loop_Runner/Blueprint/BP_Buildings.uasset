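; Building segment for the loop runner that fills itself with random buildings and triggers extension of the building row.
; The construction script adds one of four child actor variants at each of six spawn points, using each point's relative X, Y and rotation.
; Overlapping the Box asks BP_LoopRunner_GameModeBase to extend the buildings.
; GetAttachPoint exposes the Arrow's world transform as an attach point.
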(event OnComponentBeginOverlap(Box)
  (params (OverlappedComponent :type Primitive%20Component%20Object%20Reference) (OtherActor :type Actor%20Object%20Reference) (OtherComp :type Primitive%20Component%20Object%20Reference) (OtherBodyIndex :type Integer) (bFromSweep :type Boolean) (SweepResult :type Hit%20Result%20Structure%20%28by%20ref%29))
  ;[1 1 1] Extend Buildings
  (bind _asbp_loop_runner_game_mode_base (Utilities|Casting|CastToBP_LoopRunner_GameModeBase (Game|GetGameMode)))
  (Default|ExtendBuildings _asbp_loop_runner_game_mode_base))

(event EventBeginPlay)

(event Collision|EventActorBeginOverlap
  (params (OtherActor :type Actor%20Object%20Reference)))

(event EventTick
  (params (DeltaSeconds :type Float%20%28single-precision%29)))

(fn ConstructionScript
  (CallFunction|SpawnBuldings))

(fn GetAttachPoint
  ;[1 1 1] Arrow component Attach
  (return (Transformation|GetWorldTransform (Variables|Default|GetArrow))))

(fn SpawnBuldings
  (bind _sp6 (Variables|Default|GetSP6))
  (bind _sp4 (Variables|Default|GetSP4))
  (bind _sp5 (Variables|Default|GetSP5))
  (bind _sp1 (Variables|Default|GetSP1))
  (bind _sp2 (Variables|Default|GetSP2))
  (bind _sp3 (Variables|Default|GetSP3))
  (bind _returnvalue (Transformation|GetRelativeTransform _sp6))
  (bind _returnvalue_2 (Transformation|GetRelativeTransform _sp4))
  (bind _returnvalue_3 (Transformation|GetRelativeTransform _sp5))
  (bind _returnvalue_4 (Transformation|GetRelativeTransform _sp1))
  (bind _returnvalue_5 (Transformation|GetRelativeTransform _sp2))
  (bind _returnvalue_6 (Transformation|GetRelativeTransform _sp3))
  ;[1 1 1] Bulding Spawn
  (Utilities|FlowControl|Sequence
    (:then_0
      (switch int (Math|Random|RandomIntegerinRange 0 3)
        (:0
          (AddComponent|AddChildActorComponent false (Math|Transform|MakeTransform (Math|Vector|MakeVector (.x (.location _returnvalue_4)) (.y (.location _returnvalue_4)) 0.0) (.rotation _returnvalue_4) "1.000000,1.000000,1.000000")))
        (:1
          (AddComponent|AddChildActorComponent false (Math|Transform|MakeTransform (Math|Vector|MakeVector (.x (.location _returnvalue_4)) (.y (.location _returnvalue_4)) 0.0) (.rotation _returnvalue_4) "1.000000,1.000000,1.000000")))
        (:2
          (AddComponent|AddChildActorComponent false (Math|Transform|MakeTransform (Math|Vector|MakeVector (.x (.location _returnvalue_4)) (.y (.location _returnvalue_4)) 0.0) (.rotation _returnvalue_4) "1.000000,1.000000,1.000000")))
        (:3
          (AddComponent|AddChildActorComponent false (Math|Transform|MakeTransform (Math|Vector|MakeVector (.x (.location _returnvalue_4)) (.y (.location _returnvalue_4)) 0.0) (.rotation _returnvalue_4) "1.000000,1.000000,1.000000")))))
    (:then_1
      (switch int (Math|Random|RandomIntegerinRange 0 3)
        (:0
          (AddComponent|AddChildActorComponent false (Math|Transform|MakeTransform (Math|Vector|MakeVector (.x (.location _returnvalue_5)) (.y (.location _returnvalue_5)) 0.0) (.rotation _returnvalue_5) "1.000000,1.000000,1.000000")))
        (:1
          (AddComponent|AddChildActorComponent false (Math|Transform|MakeTransform (Math|Vector|MakeVector (.x (.location _returnvalue_5)) (.y (.location _returnvalue_5)) 0.0) (.rotation _returnvalue_5) "1.000000,1.000000,1.000000")))
        (:2
          (AddComponent|AddChildActorComponent false (Math|Transform|MakeTransform (Math|Vector|MakeVector (.x (.location _returnvalue_5)) (.y (.location _returnvalue_5)) 0.0) (.rotation _returnvalue_5) "1.000000,1.000000,1.000000")))
        (:3
          (AddComponent|AddChildActorComponent false (Math|Transform|MakeTransform (Math|Vector|MakeVector (.x (.location _returnvalue_5)) (.y (.location _returnvalue_5)) 0.0) (.rotation _returnvalue_5) "1.000000,1.000000,1.000000")))))
    (:then_2
      (switch int (Math|Random|RandomIntegerinRange 0 3)
        (:0
          (AddComponent|AddChildActorComponent false (Math|Transform|MakeTransform (Math|Vector|MakeVector (.x (.location _returnvalue_6)) (.y (.location _returnvalue_6)) 0.0) (.rotation _returnvalue_6) "1.000000,1.000000,1.000000")))
        (:1
          (AddComponent|AddChildActorComponent false (Math|Transform|MakeTransform (Math|Vector|MakeVector (.x (.location _returnvalue_6)) (.y (.location _returnvalue_6)) 0.0) (.rotation _returnvalue_6) "1.000000,1.000000,1.000000")))
        (:2
          (AddComponent|AddChildActorComponent false (Math|Transform|MakeTransform (Math|Vector|MakeVector (.x (.location _returnvalue_6)) (.y (.location _returnvalue_6)) 0.0) (.rotation _returnvalue_6) "1.000000,1.000000,1.000000")))
        (:3
          (AddComponent|AddChildActorComponent false (Math|Transform|MakeTransform (Math|Vector|MakeVector (.x (.location _returnvalue_6)) (.y (.location _returnvalue_6)) 0.0) (.rotation _returnvalue_6) "1.000000,1.000000,1.000000")))))
    (:then_3
      (switch int (Math|Random|RandomIntegerinRange 0 3)
        (:0
          (AddComponent|AddChildActorComponent false (Math|Transform|MakeTransform (Math|Vector|MakeVector (.x (.location _returnvalue_2)) (.y (.location _returnvalue_2)) 0.0) (.rotation _returnvalue_2) "1.000000,1.000000,1.000000")))
        (:1
          (AddComponent|AddChildActorComponent false (Math|Transform|MakeTransform (Math|Vector|MakeVector (.x (.location _returnvalue_2)) (.y (.location _returnvalue_2)) 0.0) (.rotation _returnvalue_2) "1.000000,1.000000,1.000000")))
        (:2
          (AddComponent|AddChildActorComponent false (Math|Transform|MakeTransform (Math|Vector|MakeVector (.x (.location _returnvalue_2)) (.y (.location _returnvalue_2)) 0.0) (.rotation _returnvalue_2) "1.000000,1.000000,1.000000")))
        (:3
          (AddComponent|AddChildActorComponent false (Math|Transform|MakeTransform (Math|Vector|MakeVector (.x (.location _returnvalue_2)) (.y (.location _returnvalue_2)) 0.0) (.rotation _returnvalue_2) "1.000000,1.000000,1.000000")))))
    (:then_4
      (switch int (Math|Random|RandomIntegerinRange 0 3)
        (:0
          (AddComponent|AddChildActorComponent false (Math|Transform|MakeTransform (Math|Vector|MakeVector (.x (.location _returnvalue_3)) (.y (.location _returnvalue_3)) 0.0) (.rotation _returnvalue_3) "1.000000,1.000000,1.000000")))
        (:1
          (AddComponent|AddChildActorComponent false (Math|Transform|MakeTransform (Math|Vector|MakeVector (.x (.location _returnvalue_3)) (.y (.location _returnvalue_3)) 0.0) (.rotation _returnvalue_3) "1.000000,1.000000,1.000000")))
        (:2
          (AddComponent|AddChildActorComponent false (Math|Transform|MakeTransform (Math|Vector|MakeVector (.x (.location _returnvalue_3)) (.y (.location _returnvalue_3)) 0.0) (.rotation _returnvalue_3) "1.000000,1.000000,1.000000")))
        (:3
          (AddComponent|AddChildActorComponent false (Math|Transform|MakeTransform (Math|Vector|MakeVector (.x (.location _returnvalue_3)) (.y (.location _returnvalue_3)) 0.0) (.rotation _returnvalue_3) "1.000000,1.000000,1.000000")))))
    (:then_5
      (switch int (Math|Random|RandomIntegerinRange 0 3)
        (:0
          (AddComponent|AddChildActorComponent false (Math|Transform|MakeTransform (Math|Vector|MakeVector (.x (.location _returnvalue)) (.y (.location _returnvalue)) 0.0) (.rotation _returnvalue) "1.000000,1.000000,1.000000")))
        (:1
          (AddComponent|AddChildActorComponent false (Math|Transform|MakeTransform (Math|Vector|MakeVector (.x (.location _returnvalue)) (.y (.location _returnvalue)) 0.0) (.rotation _returnvalue) "1.000000,1.000000,1.000000")))
        (:2
          (AddComponent|AddChildActorComponent false (Math|Transform|MakeTransform (Math|Vector|MakeVector (.x (.location _returnvalue)) (.y (.location _returnvalue)) 0.0) (.rotation _returnvalue) "1.000000,1.000000,1.000000")))
        (:3
          (AddComponent|AddChildActorComponent false (Math|Transform|MakeTransform (Math|Vector|MakeVector (.x (.location _returnvalue)) (.y (.location _returnvalue)) 0.0) (.rotation _returnvalue) "1.000000,1.000000,1.000000")))))))