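; Floor tile for an endless lane runner that populates itself with obstacles, coins and power-ups.
; The construction script builds per-lane arrow spawn points, shuffles them and attaches child actors, adding a power-up only once the GameMode's FloorCount passes a threshold, then resetting it.
; Box overlap tells the GameMode to extend the floor, nudges player speed up within limits and adds score.
; GetAttachPoint exposes the Arrow's world transform.
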(event OnComponentBeginOverlap(Box)
  (params (OverlappedComponent :type Primitive%20Component%20Object%20Reference) (OtherActor :type Actor%20Object%20Reference) (OtherComp :type Primitive%20Component%20Object%20Reference) (OtherBodyIndex :type Integer) (bFromSweep :type Boolean) (SweepResult :type Hit%20Result%20Structure%20%28by%20ref%29))
  ;[1 1 1] Extend Floor
  (bind _asbp_loop_runner_game_mode_base (Utilities|Casting|CastToBP_LoopRunner_GameModeBase (Game|GetGameMode)))
  (Default|ExtendFloor _asbp_loop_runner_game_mode_base)
  ;[1 1 1] Change speed
  (bind _asbp_runner_charachter (Utilities|Casting|CastToBP_RunnerCharachter (Game|GetPlayerCharacter 0)))
  (Variables|/Script/Engine.CharacterMovementComponent|SetMaxWalkSpeed (Variables|/Script/Engine.Character|GetCharacterMovement _asbp_runner_charachter) (Math|Float|Clamp(Float) (* (Variables|/Script/Engine.CharacterMovementComponent|GetMaxWalkSpeed (Variables|/Script/Engine.Character|GetCharacterMovement _asbp_runner_charachter)) 1.007) 7e+02 1.5e+03))
  ;[1 1 1] Set Current Score
  (bind _asbp_loop_runner_game_mode_base_2 (Utilities|Casting|CastToBP_LoopRunner_GameModeBase (Game|GetGameMode)))
  (Variables|/Game/Loop_Runner/Blueprint/BP_LoopRunner_GameModeBase.BP_LoopRunner_GameModeBase_C|SetCurrent%20Point _asbp_loop_runner_game_mode_base_2 (+ (* (Variables|/Game/Loop_Runner/Blueprint/BP_LoopRunner_GameModeBase.BP_LoopRunner_GameModeBase_C|GetPoints%20Multi _asbp_loop_runner_game_mode_base_2) 1) (Variables|/Game/Loop_Runner/Blueprint/BP_LoopRunner_GameModeBase.BP_LoopRunner_GameModeBase_C|GetCurrent%20Point _asbp_loop_runner_game_mode_base_2))))

(event EventBeginPlay)

(event Collision|EventActorBeginOverlap
  (params (OtherActor :type Actor%20Object%20Reference)))

(event EventTick
  (params (DeltaSeconds :type Float%20%28single-precision%29)))

(fn ConstructionScript
  (CallFunction|SetupSpawnPoints)
  (CallFunction|SpawnObstacle)
  (CallFunction|CoinSpawnPoints)
  (CallFunction|SpawnCoins)
  (CallFunction|PowerUpsSpawnPoints)
  (CallFunction|SpawnPowerUps))

(fn GetAttachPoint
  ;[1 1 1] Arrow component Attach
  (return (Transformation|GetWorldTransform (Variables|Default|GetArrow))))

(fn SetupSpawnPoints
  ;[1 1 1] Spwn Point Set
  (for _array_element (Variables|Default|GetLane%20Positon)
    (for _index (range 0 1)
      (bind _returnvalue (AddComponent|AddArrowComponent false (Math|Transform|MakeTransform (Math|Vector|MakeVector (* _index 6.5e+02) _array_element 0.0))))
      (Utilities|Array|Add (Variables|Default|GetSpawn%20Points) (Transformation|GetWorldTransform _returnvalue)))))

(fn SpawnObstacle
  ;[1 1 1] Obstacle Spawn
  (bind _output_get (LocalVariables|SetRandom%20Spawn%20Points (Variables|Default|GetSpawn%20Points)))
  (Utilities|Array|Shuffle _output_get)
  (for _index (range 0 (Math|Random|RandomIntegerinRange 0 1))
    (switch int (Math|Random|RandomIntegerinRange 0 1)
      (:0
        (AddComponent|AddChildActorComponent false (Math|Transform|MakeRelativeTransform (Utilities|Array|Get(acopy) (LocalVariables|GetRandom%20Spawn%20Points) _index) (Transformation|GetActorTransform))))
      (:1
        (AddComponent|AddChildActorComponent false (Math|Transform|MakeRelativeTransform (Utilities|Array|Get(acopy) (LocalVariables|GetRandom%20Spawn%20Points) _index) (Transformation|GetActorTransform)))))))

(fn CoinSpawnPoints
  ;[1 1 1] Coin Spawn Location Set
  (for _array_element (Variables|Default|GetLane%20Positon)
    (for _index (range 0 9)
      (bind _returnvalue (AddComponent|AddArrowComponent false (Math|Transform|MakeTransform (Math|Vector|MakeVector (* _index 75.0) _array_element 0.0))))
      (Components|Arrow|SetArrowColor(LinearColor) _returnvalue "(R=1.000000,G=0.988000,B=0.988000,A=1.000000)")
      (Utilities|Array|Add (Variables|Default|GetCSpawn%20Points) (Transformation|GetWorldTransform _returnvalue)))))

(fn SpawnCoins
  ;[1 1 1] Coin Spawn Multile Area
  (bind _output_get (LocalVariables|SetRandom%20Spawn%20Points (Variables|Default|GetCSpawn%20Points)))
  (Utilities|Array|Shuffle _output_get)
  (for _index (range 0 (Math|Random|RandomIntegerinRange 5 9))
    (switch int 0
      (:0
        (AddComponent|AddChildActorComponent false (Math|Transform|MakeRelativeTransform (Utilities|Array|Get(acopy) (LocalVariables|GetRandom%20Spawn%20Points) _index) (Transformation|GetActorTransform)))))))

(fn PowerUpsSpawnPoints
  ;[1 1 1] Coin Spawn Location Set
  (for _array_element (Variables|Default|GetLane%20Positon)
    (for _index (range 1 2)
      (bind _returnvalue (AddComponent|AddArrowComponent false (Math|Transform|MakeTransform (Math|Vector|MakeVector (* _index 2.5e+02) _array_element 0.0))))
      (Components|Arrow|SetArrowColor(LinearColor) _returnvalue "(R=1.000000,G=0.868188,B=0.000000,A=1.000000)")
      (Utilities|Array|Add (Variables|Default|GetPSpawn%20Points) (Transformation|GetWorldTransform _returnvalue)))))

(fn SpawnPowerUps
  ;[1 1 1] Magnet Spawn Multiple Area
  (bind _asbp_loop_runner_game_mode_base (Utilities|Casting|CastToBP_LoopRunner_GameModeBase (Game|GetGameMode)))
  (if (> (Variables|/Game/Loop_Runner/Blueprint/BP_LoopRunner_GameModeBase.BP_LoopRunner_GameModeBase_C|GetFloor%20Count _asbp_loop_runner_game_mode_base) 5)
    (bind _output_get (LocalVariables|SetRandom%20Spawn%20Points (Variables|Default|GetPSpawn%20Points)))
    (Utilities|Array|Shuffle _output_get)
    (switch int 0
      (:0
        (AddComponent|AddChildActorComponent false (Math|Transform|MakeRelativeTransform (Utilities|Array|Get(acopy) (LocalVariables|GetRandom%20Spawn%20Points)) (Transformation|GetActorTransform)))
        (Variables|/Game/Loop_Runner/Blueprint/BP_LoopRunner_GameModeBase.BP_LoopRunner_GameModeBase_C|SetFloor%20Count _asbp_loop_runner_game_mode_base 0)))))